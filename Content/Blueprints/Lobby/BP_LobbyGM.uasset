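; Lobby GameMode that names joining players and moves the session into the game level once everyone is ready.
; PostLogin assigns numbered nicknames through BP_LobbyPlayerState and refreshes the first local player's lobby HUD.
; TryStartGame checks every player's ready flag, copies the max player count to BP_ValheimGI, then issues ServerTravel after a short delay.
; BeginPlay enables seamless travel and reads the level name from the GameInstance; SaveConfig overrides level and player count.
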(event `TryStartGame`
  ; 모두 레디상태인지 확인
  (if (`self.IsEverybodyReady`)
    (bind _asbp_valheim_gi (cast `/Game/Blueprints/Core/BP_ValheimGI` (`GameplayStatics.GetGameInstance`)))
    (set `/Game/Blueprints/Core/BP_ValheimGI.MaxPlayerCount` (`self.Max Player Count`) _asbp_valheim_gi)
    ;; 모두 레디면 1초 대기후 인게임으로 이동
    (`KismetSystemLibrary.Delay` 1.0)
    (`KismetSystemLibrary.ExecuteConsoleCommand` (`KismetStringLibrary.Concat_StrStr` "ServerTravel" " " (`self.LevelName`)) null)))

(event `self.K2_PostLogin`
  (params (NewPlayer :type "PlayerController Object Reference"))
  ; 누군가 서버에 접속시 닉네임 설정
  (bind _asbp_lobby_player_state (cast `/Game/Blueprints/Lobby/BP_LobbyPlayerState` (`Controller.PlayerState` NewPlayer)))
  (bind _result (`/Engine/EditorBlueprintResources/StandardMacros.IncrementInt` (`self.Nickname Index`))
    (:`  `
      (`LobbyPlayerState.SetNickname` _asbp_lobby_player_state (`|FormatText` "User{0}" _result))
      (bind _asbp_lobby_hud (cast `/Game/Blueprints/Lobby/BP_LobbyHUD` (`PlayerController.GetHUD` (`GameplayStatics.GetPlayerController` 0))))
      (`/Game/Blueprints/Lobby/BP_LobbyHUD.RefreshUI` _asbp_lobby_hud))))

(event `self.ReceiveBeginPlay`
  (set `self.bUseSeamlessTravel` true)
  (bind _asbp_valheim_gi (cast `/Game/Blueprints/Core/BP_ValheimGI` (`GameplayStatics.GetGameInstance`)))
  (set `self.LevelName` (`ValheimGI.LevelName` _asbp_valheim_gi)))

(fn `IsEverybodyReady`
  (returns (bIsReady :type Boolean))
  (for _array_element (`GameStateBase.PlayerArray` (`GameplayStatics.GetGameState`))
    (bind _asbp_lobby_player_state (cast `/Game/Blueprints/Lobby/BP_LobbyPlayerState` _array_element))
    (if (not (`/Game/Blueprints/Lobby/BP_LobbyPlayerState.bIsReady` _asbp_lobby_player_state))
      (return false)))
  (return true))

(fn `SaveConfig`
  (params (InLevelName :type String) (InMaxPlayerCount :type Integer))
  (set `self.LevelName` InLevelName)
  (set `self.Max Player Count` InMaxPlayerCount))

(fn `UserConstructionScript`)