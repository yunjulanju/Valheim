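; BP_MosnterController is the AI controller for a monster, driving it with a behavior tree and sight perception.
; On possess it initializes the BB_Monster blackboard and runs BT_Monster.
; Perception updates from the sight sense set the blackboard's Target to the seen actor and clear it when sight is lost; other senses are ignored.
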(event `self.ReceiveBeginPlay`)

(event `self.ReceivePossess`
  (params (PossessedPawn :type "Pawn Object Reference"))
  (bind _blackboardcomponent (`self.UseBlackboard` "/Game/Blueprints/Monster/AI/BB_Monster.BB_Monster"))
  (set `self.Blackboard Component` _blackboardcomponent)
  (`self.RunBehaviorTree` "/Game/Blueprints/Monster/AI/BT_Monster.BT_Monster"))

(event `self.AIPerception.OnTargetPerceptionUpdated`
  (params (Actor :type "Actor Object Reference") (Stimulus :type "AIStimulus Structure"))
  (bind _returnvalue (`AIPerceptionSystem.GetSenseClassForStimulus` Stimulus))
  (if (== _returnvalue "/Script/AIModule.AISense_Sight")
    (if (`.bSuccessfullySensed` (break `AIStimulus` Stimulus))
      (`BlackboardComponent.SetValueAsObject` (`self.Blackboard Component`) "Target" Actor)
      (else
        (`BlackboardComponent.SetValueAsObject` (`self.Blackboard Component`) "Target" null)))))

(fn `UserConstructionScript`)