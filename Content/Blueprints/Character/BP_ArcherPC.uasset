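; Player controller for the archer character, turning Enhanced Input actions into pawn movement, camera look and attacks.
; On BeginPlay it adds the default mapping context and caches the controlled pawn as a BP_Archer reference.
; Move input follows control-rotation yaw, and look input drives yaw and inverted-value pitch on the controller.
; Crouch and jump start on press and end on release or cancel, while attack calls the archer's CallAttack.
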(event `self.ReceiveBeginPlay`
  (`EnhancedInputSubsystemInterface.AddMappingContext` (subsystem `EnhancedInputLocalPlayerSubsystem`) "/Game/Input/IMC_Default.IMC_Default" 0 (struct))
  (bind _asbp_archer (cast `/Game/Blueprints/Character/BP_Archer` (`self.K2_GetPawn`)))
  (set `self.ArcherRef` _asbp_archer))

(event `EnhancedInput|/Game/Input/Actions/IA_Move`
  (params (ActionValue :type "Vector2D Structure") (ElapsedSeconds :type "Float (double-precision)") (TriggeredSeconds :type "Float (double-precision)") (InputAction :type "InputAction Object Reference" :default "/Game/Input/Actions/IA_Move.IA_Move"))
  (bind (_returnvalue_roll _returnvalue_pitch _returnvalue_yaw) (`KismetMathLibrary.BreakRotator` (`self.GetControlRotation`)))
  (bind _archerref (`self.ArcherRef`))
  (bind (_returnvalue_x _returnvalue_y) (`KismetMathLibrary.BreakVector` (`KismetMathLibrary.GetForwardVector` (`KismetMathLibrary.MakeRotator` _returnvalue_roll 0.0 _returnvalue_yaw))))
  (bind (_returnvalue_x_2 _returnvalue_y_2) (`KismetMathLibrary.BreakVector` (`KismetMathLibrary.GetRightVector` (`KismetMathLibrary.MakeRotator` _returnvalue_roll 0.0 _returnvalue_yaw))))
  (:`Triggered`
    (`|ExecutionSequence`
      (:`then_0`
        (`Pawn.AddMovementInput` _archerref (`KismetMathLibrary.MakeVector` _returnvalue_x _returnvalue_y) ActionValue_X false))
      (:`then_1`
        (`Pawn.AddMovementInput` _archerref (`KismetMathLibrary.MakeVector` _returnvalue_x_2 _returnvalue_y_2) ActionValue_Y false)))))

(event `EnhancedInput|/Game/Input/Actions/IA_Crouch`
  (params (ActionValue :type Boolean) (ElapsedSeconds :type "Float (double-precision)") (TriggeredSeconds :type "Float (double-precision)") (InputAction :type "InputAction Object Reference" :default "/Game/Input/Actions/IA_Crouch.IA_Crouch"))
  (bind _archerref (`self.ArcherRef`))
  (:`Started`
    (`Character.Crouch` _archerref))
  (:`Canceled`
    (`Character.UnCrouch` _archerref :!label _label))
  (:`Completed`
    (goto _label)))

(event `EnhancedInput|/Game/Input/Actions/IA_Jump`
  (params (ActionValue :type Boolean) (ElapsedSeconds :type "Float (double-precision)") (TriggeredSeconds :type "Float (double-precision)") (InputAction :type "InputAction Object Reference" :default "/Game/Input/Actions/IA_Jump.IA_Jump"))
  (bind _archerref (`self.ArcherRef`))
  (:`Started`
    (`Character.Jump` _archerref))
  (:`Canceled`
    (`Character.StopJumping` _archerref :!label _label_2))
  (:`Completed`
    (goto _label_2)))

(event `EnhancedInput|/Game/Input/Actions/IA_Look`
  (params (ActionValue :type "Vector2D Structure") (ElapsedSeconds :type "Float (double-precision)") (TriggeredSeconds :type "Float (double-precision)") (InputAction :type "InputAction Object Reference" :default "/Game/Input/Actions/IA_Look.IA_Look"))
  (:`Triggered`
    (`self.AddYawInput` ActionValue_X)
    (`self.AddPitchInput` (* ActionValue_Y -1.0))))

(event `EnhancedInput|/Game/Input/Actions/IA_Attack`
  (params (ActionValue :type Boolean) (ElapsedSeconds :type "Float (double-precision)") (TriggeredSeconds :type "Float (double-precision)") (InputAction :type "InputAction Object Reference" :default "/Game/Input/Actions/IA_Attack.IA_Attack"))
  (:`Triggered`
    (`/Game/Blueprints/Character/BP_Archer.Call_Attack` (`self.ArcherRef`))))

(fn `UserConstructionScript`)