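; Lobby player state that holds a player's nickname and ready flag and keeps the lobby UI in sync.
; BeginPlay, destruction and the server-to-all ready event each refresh the UI through the local controller's BP_LobbyHUD.
; CopyProperties passes Nickname on only when the new player state casts to BP_LobbyPlayerState.
; A server-to-client kick event sends the player back to the Title level.
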(event `self.ReceiveBeginPlay`
  ; 접속한이후
  (`self.RefreshLobbyUI`)
  (add `Actor.OnDestroyed` (delegate `OnDestroyed_Event`)))

(event `OnDestroyed_Event`
  (params (DestroyedActor :type "Actor Object Reference"))
  (`self.RefreshLobbyUI`))

(event `self.ReceiveCopyProperties`
  (params (NewPlayerState :type "PlayerState Object Reference"))
  ; 로비 플레이어스테이트의 정보를 인게임 플레이어스테이트로 전달
  ;; 서버에서만 호출
  (`parent.ReceiveCopyProperties` NewPlayerState)
  (bind _asbp_lobby_player_state (cast `/Game/Blueprints/Lobby/BP_LobbyPlayerState` NewPlayerState))
  (set `LobbyPlayerState.Nickname` (`self.Nickname`) _asbp_lobby_player_state))

(event `S2M_HandleReadyButton`
  ; 서버가 레디를 누른애를 모두에게 알려줌, 갱신하라고 함
  (set `self.bIsReady` true)
  (`self.RefreshLobbyUI`))

(event `S2C_KickedByServer`
  ; 강제추방(맵 이동 요청)
  (`GameplayStatics.OpenLevelBySoftObjectPtr` "/Game/Maps/Title.Title"))

(fn `RefreshLobbyUI`
  (bind _returnvalue (`GameplayStatics.GetPlayerController` 0))
  (`/Engine/EditorBlueprintResources/StandardMacros.IsValid` _returnvalue
    (:`Is Valid`
      (bind _asbp_lobby_hud (cast `/Game/Blueprints/Lobby/BP_LobbyHUD` (`PlayerController.GetHUD` _returnvalue)))
      (`/Game/Blueprints/Lobby/BP_LobbyHUD.RefreshUI` _asbp_lobby_hud))))

(fn `UserConstructionScript`)