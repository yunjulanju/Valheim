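; BP_Velo is the Velo monster Blueprint, handling its attack and death animations.
; CallAttack sets the Attacking state unless already attacking or moving, while CallDeathAnimation uses a flag, never cleared here, to block repeat calls.
; Both pass through C2S events to S2M events, named as a client-to-server-to-multicast relay, which play the matching montages.
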(event `self.CallAttack`
  (bind _currentstate (`self.CurrentState`))
  (if (not (or (`|EnumEquality` _currentstate "Attacking") (`|EnumEquality` _currentstate "Moving")))
    (set `self.CurrentState` "Attacking")
    (`self.C2S_CallAttackAnim`)))

(event `C2S_CallAttackAnim`
  (`self.S2M_CallAttackAnim`))

(event `S2M_CallAttackAnim`
  (`self.PlayAnimMontage` "/Game/Blueprints/Monster/Animation/velo/AM_Velo_Attack.AM_Velo_Attack"))

(event `self.CallDeathAnimation`
  (if (not (`self.bIsPlayingAnim`))
    (set `self.bIsPlayingAnim` true)
    (`self.C2S_DeathAnimation`)))

(event `C2S_DeathAnimation`
  (`self.S2M_DeathAnim`))

(event `S2M_DeathAnim`
  (`self.PlayAnimMontage` "/Game/Blueprints/Monster/Animation/velo/AM_Velo_Death.AM_Velo_Death"))

(fn `UserConstructionScript`
  (`parent.UserConstructionScript`))