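; BP_LobbyPC is the lobby player controller that relays ready-button presses and nickname changes to the server.
; Local handler events call C2S events, which reach BP_LobbyPlayerState through the controlled pawn.
; On ready, the server has the player state broadcast the change through its S2M event, then asks BP_LobbyGM to try starting the game.
; Nickname changes are written directly to the player state's Nickname.
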(event `HandleReadyButton`
  ; 서버로 레디버튼 눌렸음을 전달
  (`self.C2S_HandelReadyButton`))

(event `C2S_HandelReadyButton`
  ; 서버에서 눌른 폰에 대한 플레이어 스테이트 가져와서 레디 눌렸음을 모두에게 알려줌
  (if (`KismetSystemLibrary.IsServer`)
    (bind _asbp_lobby_player_state (cast `/Game/Blueprints/Lobby/BP_LobbyPlayerState` (`Pawn.PlayerState` (`self.K2_GetPawn`))))
    (`/Game/Blueprints/Lobby/BP_LobbyPlayerState.S2M_HandleReadyButton` _asbp_lobby_player_state)
    (bind _asbp_lobby_gm (cast `/Game/Blueprints/Lobby/BP_LobbyGM` (`GameplayStatics.GetGameMode`)))
    ; Try Start GAme
    (`/Game/Blueprints/Lobby/BP_LobbyGM.TryStartGame` _asbp_lobby_gm)))

(event `HandleChangeNickname`
  (params (Nickname :type Text))
  ; 닉네임
  (`self.C2S_HandleChangeNickname` Nickname))

(event `C2S_HandleChangeNickname`
  (params (Nickname :type Text))
  ; 닉네임
  (bind _asbp_lobby_player_state (cast `/Game/Blueprints/Lobby/BP_LobbyPlayerState` (`Pawn.PlayerState` (`self.K2_GetPawn`))))
  (set `LobbyPlayerState.Nickname` Nickname _asbp_lobby_player_state))

(fn `UserConstructionScript`)