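; BP_Stega is the Stega monster Blueprint, supplying its attack and death animations.
; CallAttack and CallDeathAnimation forward to C2S-prefixed events, whose naming suggests client-to-server RPCs.
; The attack event plays its montage directly, while the death event plays its montage only when the mesh reports it is not playing.
; BeginPlay, overlap and Tick are disabled stubs, and the construction script only calls its parent.
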(event `self.CallAttack`
  (`self.C2S_CallAttackAnim`))

(event `C2S_CallAttackAnim`
  (`self.PlayAnimMontage` "/Game/Blueprints/Monster/Animation/Stega/AM_Stega_Attack.AM_Stega_Attack"))

(event `self.CallDeathAnimation`
  (`self.C2S_DeathAnimation`))

(event `C2S_DeathAnimation`
  (bind _mesh (`self.Mesh`))
  (if (not (`SkeletalMeshComponent.IsPlaying` _mesh))
    (`|PlayMontage` _mesh "/Game/Blueprints/Monster/Animation/Stega/AM_Steaga_Death.AM_Steaga_Death")))

(fn `UserConstructionScript`
  (`parent.UserConstructionScript`))